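; Prototype enemy actor that spins in place and destroys projectiles that touch it.
; Its Box overlap prints a debug message, then destroys the other actor if it casts to BP_Projectile.
; The flattened-location check before destruction compares the enemy's own position to itself, so it always passes.
; Tick decrements yaw by a fixed step each frame, making the spin frame-rate dependent.
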(event `self.ReceiveBeginPlay`)

(event `self.Box.OnComponentBeginOverlap`
  (params (OverlappedComponent :type "PrimitiveComponent Object Reference") (OtherActor :type "Actor Object Reference") (OtherComp :type "PrimitiveComponent Object Reference") (OtherBodyIndex :type Integer) (bFromSweep :type Boolean) (SweepResult :type "HitResult Structure (by ref)"))
  (`KismetSystemLibrary.PrintString` "enemy collided")
  (bind _asbp_projectile (cast `/Game/Blueprints/Player/BP_Projectile` OtherActor))
  (if (== (`KismetMathLibrary.MakeVector` (.x (`self.K2_GetActorLocation`)) (.y (`self.K2_GetActorLocation`))) (`KismetMathLibrary.MakeVector` (.x (`self.K2_GetActorLocation`)) (.y (`self.K2_GetActorLocation`))) :`ErrorTolerance` 1000.0)
    (`self.K2_DestroyActor` _asbp_projectile)))

(event `self.ReceiveTick`
  (params (DeltaSeconds :type "Float (single-precision)"))
  (bind (_returnvalue_roll _returnvalue_pitch _returnvalue_yaw) (`KismetMathLibrary.BreakRotator` (`self.K2_GetActorRotation`)))
  (`self.K2_SetActorRotation` (`KismetMathLibrary.MakeRotator` _returnvalue_roll _returnvalue_pitch (+ _returnvalue_yaw -1.0))))

(fn `UserConstructionScript`)