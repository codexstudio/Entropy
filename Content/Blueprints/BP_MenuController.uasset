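; Player controller for the start menu that handles local multiplayer sign-in and character class selection.
; Each controller registers with BP_GameInstance; any key press finds the pressing controller, sets the active player, updates the player-select UI and forwards active-player keys to StartMenuGameMode.
; On the select screen, signed-in players cycle class sprites with wraparound, saving picks per controller ID.
; Only the active player can start the level load.
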(event `self.ReceiveBeginPlay`
  (bind _asbp_game_instance (cast `/Game/Blueprints/BP_GameInstance` (`GameplayStatics.GetGameInstance`)))
  (`KismetArrayLibrary.Array_Add` (`/Game/Blueprints/BP_GameInstance.MenuPCArray` _asbp_game_instance) self))

(event `Key|AnyKey`
  (params (Key :type "Key Structure"))
  ;[1 1 1] Go through the cases of any key
  (:`Pressed`
    (bind _asbp_game_instance (cast `/Game/Blueprints/BP_GameInstance` (`GameplayStatics.GetGameInstance`)))
    (for _array_element (`/Game/Blueprints/BP_GameInstance.MenuPCArray` _asbp_game_instance)
      (if (`self.WasInputKeyJustPressed` _array_element Key)
        (bind _returnvalue (`GameplayStatics.GetPlayerControllerID` _array_element))
        (bind (_output _activewasset) (`/Game/Blueprints/BP_GameInstance.SetActivePlayer` _asbp_game_instance _returnvalue))
        (if _activewasset
          (set `self.bIsSignedIn` true))
        (bind _asstart_menu_game_mode (cast `/Game/UI/StartMenuGameMode` (`GameplayStatics.GetGameMode`)))
        (bind _startmenu (`/Game/UI/StartMenuGameMode.StartMenu` _asstart_menu_game_mode))
        (bind _switcher (`/Game/UI/MainMenuWidgets/StartMenuUI.Switcher` _startmenu))
        (bind _returnvalue_2 (`WidgetSwitcher.GetActiveWidgetIndex` _switcher))
        (if (or (== _output (`/Game/Blueprints/BP_GameInstance.ActivePlayer` _asbp_game_instance)) (== _returnvalue_2 1))
          (`/Game/UI/MainMenuWidgets/PlayerSelectUI.SetPlayerSignedIn` (`/Game/UI/MainMenuWidgets/StartMenuUI.PlayerSelectUI` _startmenu) _output))
        (if (== 5 _returnvalue_2)
          (`WidgetSwitcher.SetActiveWidgetIndex` _switcher 0)
          (else
            (bind _returnvalue_3 (`GameplayStatics.GetPlayerControllerID` _array_element))
            (if (== _returnvalue_3 _output)
              (`/Game/UI/StartMenuGameMode.Keypress` _asstart_menu_game_mode Key _output))))))))

(event `Key|S`
  (params (Key :type "Key Structure"))
  ;[1 1 1] Start Game Player Select
  (:`Pressed`
    (bind _asstart_menu_game_mode (cast `/Game/UI/StartMenuGameMode` (`GameplayStatics.GetGameMode`) :!label _label))
    (bind _asbp_game_instance (cast `/Game/Blueprints/BP_GameInstance` (`GameplayStatics.GetGameInstance`)))
    (bind _returnvalue (`GameplayStatics.GetPlayerControllerID` self))
    (if (and (== _returnvalue (`/Game/Blueprints/BP_GameInstance.ActivePlayer` _asbp_game_instance)) (== (`WidgetSwitcher.ActiveWidgetIndex` (`/Game/UI/MainMenuWidgets/StartMenuUI.Switcher` (`/Game/UI/StartMenuGameMode.StartMenu` _asstart_menu_game_mode))) 1))
      (`/Game/UI/StartMenuGameMode.LoadLevel` _asstart_menu_game_mode))))

(event `Key|Gamepad_Special_Right`
  (params (Key :type "Key Structure"))
  ;[1 1 1] Start Game Player Select
  (:`Pressed`
    (goto _label)))

(event `Key|Gamepad_RightShoulder`
  (params (Key :type "Key Structure"))
  (bind _characterselect (`self.CharacterSelect`))
  ;[1 1 1] Change Class in Player Select Going Right
  (:`Pressed`
    (bind _asstart_menu_game_mode (cast `/Game/UI/StartMenuGameMode` (`GameplayStatics.GetGameMode`) :!label _label_2))
    (bind _startmenu (`/Game/UI/StartMenuGameMode.StartMenu` _asstart_menu_game_mode))
    (if (== (`WidgetSwitcher.ActiveWidgetIndex` (`/Game/UI/MainMenuWidgets/StartMenuUI.Switcher` _startmenu)) 1)
      (bind _returnvalue (`GameplayStatics.GetPlayerControllerID` self))
      (if (`self.bIsSignedIn`)
        (bind _asbp_game_instance (cast `/Game/Blueprints/BP_GameInstance` (`GameplayStatics.GetGameInstance`)))
        (switch `int` _returnvalue
          (:`0`
            (bind _result (`/Engine/EditorBlueprintResources/StandardMacros.IncrementInt` _characterselect)
              (:`  `
                (bind _playerspritearray (`/Game/Blueprints/BP_GameInstance.PlayerSpriteArray` _asbp_game_instance))
                (bind _returnvalue_2 (`KismetArrayLibrary.Array_Length` _playerspritearray))
                (if (>= _result _returnvalue_2)
                  (bind _output_get (set `self.CharacterSelect` 0)))
                (bind _playerselectui (`/Game/UI/MainMenuWidgets/StartMenuUI.PlayerSelectUI` _startmenu))
                (bind _output (`|GetArrayItem` _playerspritearray _characterselect))
                (`Image.SetBrush` (`/Game/UI/MainMenuWidgets/PlayerSelectUI.PlayerOneImage` _playerselectui) _output)
                (bind _returnvalue_3 (`GameplayStatics.GetPlayerControllerID` self))
                (bind _asbp_game_instance_2 (cast `/Game/Blueprints/BP_GameInstance` (`GameplayStatics.GetGameInstance`)))
                (`BlueprintMapLibrary.Map_Add` (`/Game/Blueprints/BP_GameInstance.PCSelectMap` _asbp_game_instance_2) _returnvalue_3 _output_get))))
          (:`1`
            (bind _result_2 (`/Engine/EditorBlueprintResources/StandardMacros.IncrementInt` _characterselect)
              (:`  `
                (if (>= _result_2 _returnvalue_2)
                  (bind _output_get_2 (set `self.CharacterSelect` 0)))
                (`Image.SetBrush` (`/Game/UI/MainMenuWidgets/PlayerSelectUI.PlayerTwoImage` _playerselectui) _output)
                (bind _returnvalue_4 (`GameplayStatics.GetPlayerControllerID` self))
                (bind _asbp_game_instance_3 (cast `/Game/Blueprints/BP_GameInstance` (`GameplayStatics.GetGameInstance`)))
                (`BlueprintMapLibrary.Map_Add` (`/Game/Blueprints/BP_GameInstance.PCSelectMap` _asbp_game_instance_3) _returnvalue_4 _output_get_2))))
          (:`2`
            (bind _result_3 (`/Engine/EditorBlueprintResources/StandardMacros.IncrementInt` _characterselect)
              (:`  `
                (if (>= _result_3 _returnvalue_2)
                  (bind _output_get_3 (set `self.CharacterSelect` 0)))
                (`Image.SetBrush` (`/Game/UI/MainMenuWidgets/PlayerSelectUI.PlayerThreeImage` _playerselectui) _output)
                (bind _returnvalue_5 (`GameplayStatics.GetPlayerControllerID` self))
                (bind _asbp_game_instance_4 (cast `/Game/Blueprints/BP_GameInstance` (`GameplayStatics.GetGameInstance`)))
                (`BlueprintMapLibrary.Map_Add` (`/Game/Blueprints/BP_GameInstance.PCSelectMap` _asbp_game_instance_4) _returnvalue_5 _output_get_3))))
          (:`3`
            (bind _result_4 (`/Engine/EditorBlueprintResources/StandardMacros.IncrementInt` _characterselect)
              (:`  `
                (if (>= _result_4 _returnvalue_2)
                  (bind _output_get_4 (set `self.CharacterSelect` 0)))
                (`Image.SetBrush` (`/Game/UI/MainMenuWidgets/PlayerSelectUI.PlayerFourImage` _playerselectui) _output)
                (bind _returnvalue_6 (`GameplayStatics.GetPlayerControllerID` self))
                (bind _asbp_game_instance_5 (cast `/Game/Blueprints/BP_GameInstance` (`GameplayStatics.GetGameInstance`)))
                (`BlueprintMapLibrary.Map_Add` (`/Game/Blueprints/BP_GameInstance.PCSelectMap` _asbp_game_instance_5) _returnvalue_6 _output_get_4)))))))))

(event `Key|Right`
  (params (Key :type "Key Structure"))
  ;[1 1 1] Change Class in Player Select Going Right
  (:`Pressed`
    (goto _label_2)))

(event `Key|Gamepad_DPad_Right`
  (params (Key :type "Key Structure"))
  ;[1 1 1] Change Class in Player Select Going Right
  (:`Pressed`
    (goto _label_2)))

(event `Key|Gamepad_LeftShoulder`
  (params (Key :type "Key Structure"))
  (bind _characterselect (`self.CharacterSelect`))
  ;[1 1 1] Change Class Player Select Going Left
  (:`Pressed`
    (bind _asstart_menu_game_mode (cast `/Game/UI/StartMenuGameMode` (`GameplayStatics.GetGameMode`) :!label _label_3))
    (bind _startmenu (`/Game/UI/StartMenuGameMode.StartMenu` _asstart_menu_game_mode))
    (if (== (`WidgetSwitcher.ActiveWidgetIndex` (`/Game/UI/MainMenuWidgets/StartMenuUI.Switcher` _startmenu)) 1)
      (bind _returnvalue (`GameplayStatics.GetPlayerControllerID` self))
      (if (`self.bIsSignedIn`)
        (bind _asbp_game_instance (cast `/Game/Blueprints/BP_GameInstance` (`GameplayStatics.GetGameInstance`)))
        (switch `int` _returnvalue
          (:`0`
            (bind _result (`/Engine/EditorBlueprintResources/StandardMacros.DecrementInt` _characterselect)
              (:`  `
                (if (< _result 0)
                  (bind _playerspritearray (`/Game/Blueprints/BP_GameInstance.PlayerSpriteArray` _asbp_game_instance))
                  (bind _returnvalue_2 (- (`KismetArrayLibrary.Array_Length` _playerspritearray) 1))
                  (bind _output_get (set `self.CharacterSelect` _returnvalue_2)))
                (bind _playerselectui (`/Game/UI/MainMenuWidgets/StartMenuUI.PlayerSelectUI` _startmenu))
                (bind _output (`|GetArrayItem` _playerspritearray _characterselect))
                (`Image.SetBrush` (`/Game/UI/MainMenuWidgets/PlayerSelectUI.PlayerOneImage` _playerselectui) _output)
                (bind _returnvalue_3 (`GameplayStatics.GetPlayerControllerID` self))
                (bind _asbp_game_instance_2 (cast `/Game/Blueprints/BP_GameInstance` (`GameplayStatics.GetGameInstance`)))
                (`BlueprintMapLibrary.Map_Add` (`/Game/Blueprints/BP_GameInstance.PCSelectMap` _asbp_game_instance_2) _returnvalue_3 _output_get))))
          (:`1`
            (bind _result_2 (`/Engine/EditorBlueprintResources/StandardMacros.DecrementInt` _characterselect)
              (:`  `
                (if (< _result_2 0)
                  (bind _output_get_2 (set `self.CharacterSelect` _returnvalue_2)))
                (`Image.SetBrush` (`/Game/UI/MainMenuWidgets/PlayerSelectUI.PlayerTwoImage` _playerselectui) _output)
                (bind _returnvalue_4 (`GameplayStatics.GetPlayerControllerID` self))
                (bind _asbp_game_instance_3 (cast `/Game/Blueprints/BP_GameInstance` (`GameplayStatics.GetGameInstance`)))
                (`BlueprintMapLibrary.Map_Add` (`/Game/Blueprints/BP_GameInstance.PCSelectMap` _asbp_game_instance_3) _returnvalue_4 _output_get_2))))
          (:`2`
            (bind _result_3 (`/Engine/EditorBlueprintResources/StandardMacros.DecrementInt` _characterselect)
              (:`  `
                (if (< _result_3 0)
                  (bind _output_get_3 (set `self.CharacterSelect` _returnvalue_2)))
                (`Image.SetBrush` (`/Game/UI/MainMenuWidgets/PlayerSelectUI.PlayerThreeImage` _playerselectui) _output)
                (bind _returnvalue_5 (`GameplayStatics.GetPlayerControllerID` self))
                (bind _asbp_game_instance_4 (cast `/Game/Blueprints/BP_GameInstance` (`GameplayStatics.GetGameInstance`)))
                (`BlueprintMapLibrary.Map_Add` (`/Game/Blueprints/BP_GameInstance.PCSelectMap` _asbp_game_instance_4) _returnvalue_5 _output_get_3))))
          (:`3`
            (bind _result_4 (`/Engine/EditorBlueprintResources/StandardMacros.DecrementInt` _characterselect)
              (:`  `
                (if (< _result_4 0)
                  (bind _output_get_4 (set `self.CharacterSelect` _returnvalue_2)))
                (`Image.SetBrush` (`/Game/UI/MainMenuWidgets/PlayerSelectUI.PlayerFourImage` _playerselectui) _output)
                (bind _returnvalue_6 (`GameplayStatics.GetPlayerControllerID` self))
                (bind _asbp_game_instance_5 (cast `/Game/Blueprints/BP_GameInstance` (`GameplayStatics.GetGameInstance`)))
                (`BlueprintMapLibrary.Map_Add` (`/Game/Blueprints/BP_GameInstance.PCSelectMap` _asbp_game_instance_5) _returnvalue_6 _output_get_4)))))))))

(event `Key|Left`
  (params (Key :type "Key Structure"))
  ;[1 1 1] Change Class Player Select Going Left
  (:`Pressed`
    (goto _label_3)))

(event `Key|Gamepad_DPad_Left`
  (params (Key :type "Key Structure"))
  ;[1 1 1] Change Class Player Select Going Left
  (:`Pressed`
    (goto _label_3)))

(fn `UserConstructionScript`)