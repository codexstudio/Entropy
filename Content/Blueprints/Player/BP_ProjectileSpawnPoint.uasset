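; BP_ProjectileSpawnPoint is a player weapon actor that fires BP_Projectile automatically while its trigger is held.
; PullTrigger passes through a DoOnce gate to fire immediately, then starts a looping timer by function name at an interval set by FireRate.
; Each Fire spawns a projectile at the ProjectileSpawnPoint component's world transform.
; ReleaseTrigger clears the timer and resets the gate.
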(event `PullTrigger`
  (`/Engine/EditorBlueprintResources/StandardMacros.DoOnce` false :!label _label
    (:`Completed`
      (`self.Fire`)
      (`KismetSystemLibrary.K2_SetTimer` null "Fire" (/ 1.0 (`self.FireRate`)) true))))

(event `ReleaseTrigger`
  (`KismetSystemLibrary.K2_ClearTimer` null "Fire")
  (goto _label :!via `Reset`))

(event `Fire`
  (`|SpawnActorFromClass` "/Game/Blueprints/Player/BP_Projectile.BP_Projectile_C" (`SceneComponent.K2_GetComponentToWorld` (`self.ProjectileSpawnPoint`)) "Undefined" "OverrideRootScale" null null))

(fn `UserConstructionScript`)