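; BP_Character_ADC is a character Blueprint that rotates with aim-axis input and fires through a spawned projectile spawn point actor.
; On BeginPlay it spawns BP_ProjectileSpawnPoint at the spawn point component and attaches it there.
; Both aim axes share one path that sets rotation via FindLookAtRotation between the input vector and actor location, then calls PullTrigger.
; Dead-zone checks and ReleaseTrigger are unconnected, so firing is never gated or released here.
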(event `self.ReceiveBeginPlay`
  ;[1 1 1] Set Projectile Spawn Point
  (bind _returnvalue (`|SpawnActorFromClass` "/Game/Blueprints/Player/BP_ProjectileSpawnPoint.BP_ProjectileSpawnPoint_C" (`SceneComponent.K2_GetComponentToWorld` (`self.ProjectileSpawnPoint`)) "Undefined" "OverrideRootScale" null null))
  (bind _output_get (set `self.Projectile Spawn Point` _returnvalue))
  (`self.K2_AttachToComponent` _output_get (`self.ProjectileSpawnPoint`) "None" "SnapToTarget" "KeepWorld" "KeepWorld" true))

(event `InputAxis|AimUp`
  (params (AxisValue :type "Float (single-precision)"))
  ;[1 1 1] Rotating the Character and Firing
  (`self.K2_SetActorRotation` (`KismetMathLibrary.FindLookAtRotation` (`KismetMathLibrary.MakeVector` (`self.GetInputAxisValue`) (`self.GetInputAxisValue`)) (`self.K2_GetActorLocation`)) :!label _label)
  (`/Game/Blueprints/Player/BP_ProjectileSpawnPoint.PullTrigger` (`self.Projectile Spawn Point`)))

(event `InputAxis|AimRight`
  (params (AxisValue :type "Float (single-precision)"))
  ;[1 1 1] Rotating the Character and Firing
  (goto _label))

(fn `UserConstructionScript`)