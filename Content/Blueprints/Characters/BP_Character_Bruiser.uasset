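; BP_Character_Bruiser is the Bruiser character Blueprint, which updates the shared count of living players and triggers game over.
; IsAliveAgain increments PlayersAlive on BP_GameInstance, while IsPlayerAlive decrements it despite its query-like name.
; When the decrement brings the count to zero or below, IsPlayerAlive opens the GameOverMenu level.
; The construction script is empty.
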(event `self.IsAliveAgain`
  (bind _asbp_game_instance (cast `/Game/Blueprints/BP_GameInstance` (`GameplayStatics.GetGameInstance`)))
  (set `/Game/Blueprints/BP_GameInstance.PlayersAlive` (+ (`/Game/Blueprints/BP_GameInstance.PlayersAlive` _asbp_game_instance) 1) _asbp_game_instance))

(event `self.isPlayerAlive`
  (bind _asbp_game_instance (cast `/Game/Blueprints/BP_GameInstance` (`GameplayStatics.GetGameInstance`)))
  (bind _output_get (set `/Game/Blueprints/BP_GameInstance.PlayersAlive` (- (`/Game/Blueprints/BP_GameInstance.PlayersAlive` _asbp_game_instance) 1) _asbp_game_instance))
  (if (<= _output_get 0)
    (`GameplayStatics.OpenLevel` "GameOverMenu")))

(fn `UserConstructionScript`)