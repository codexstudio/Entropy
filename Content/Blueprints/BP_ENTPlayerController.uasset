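; BP_ENTPlayerController is a player controller that handles join and start input for a player select screen.
; The gamepad bottom face button toggles IsReady, then updates the player select widget held by BP_GameInstance with this controller and a joined or prompt text.
; The gamepad special right button calls StartGame on BP_GameInstance, passing this controller, with no ready check in this Blueprint.
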(event `Key|Gamepad_FaceButton_Bottom`
  (params (Key :type "Key Structure"))
  (:`Pressed`
    (`KismetSystemLibrary.PrintString` "Signed  In")
    (bind _output_get (set `self.IsReady` (not (`self.IsReady`))))
    (bind _asbp_game_instance (cast `/Game/Blueprints/BP_GameInstance` (`GameplayStatics.GetGameInstance`)))
    (if _output_get
      (bind _playerselectwidget (`/Game/Blueprints/BP_GameInstance.PlayerSelectWidget` _asbp_game_instance))
      (`/Game/UI/PlayerSelectUI.Update Players` _playerselectwidget self "Player Joined")
      (else
        (`/Game/UI/PlayerSelectUI.Update Players` _playerselectwidget self "Press A to Join")))))

(event `Key|Gamepad_Special_Right`
  (params (Key :type "Key Structure"))
  (:`Pressed`
    (bind _asbp_game_instance (cast `/Game/Blueprints/BP_GameInstance` (`GameplayStatics.GetGameInstance`)))
    (`/Game/Blueprints/BP_GameInstance.StartGame` _asbp_game_instance self)))

(fn `UserConstructionScript`)