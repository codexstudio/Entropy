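; Game mode that spawns each player as their selected character class and color variant.
; SpawnDefaultPawnFor looks up the player controller's ID in BP_GameInstance's PCSelectMap, returning no pawn if absent.
; The selection index picks ADC, Assassin, Bruiser or Tank in four colors, spawned at the start spot with a matching sprite.
; Pink, blue and green Tank selections spawn BP_Character_Bruiser with Tank sprites; only red spawns BP_Character_Tank.
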(event `self.ReceiveBeginPlay`)

(fn `SpawnDefaultPawnFor`
  (params (NewPlayer :type "Controller Object Reference") (StartSpot :type "Actor Object Reference"))
  (returns (ReturnValue :type "Pawn Object Reference"))
  (bind _returnvalue (`self.GetTransform` StartSpot))
  (bind _asbp_game_instance (cast `/Game/Blueprints/BP_GameInstance` (`GameplayStatics.GetGameInstance`)))
  (bind _asplayer_controller (cast `PlayerController` NewPlayer))
  (bind _returnvalue_2 (`GameplayStatics.GetPlayerControllerID` _asplayer_controller))
  (bind (_value _returnvalue_3) (`BlueprintMapLibrary.Map_Find` (`/Game/Blueprints/BP_GameInstance.PCSelectMap` _asbp_game_instance) _returnvalue_2))
  (if _returnvalue_3
    (switch `int` _value
      (:`0`
        (bind _returnvalue_4 (`|SpawnActorFromClass` "/Game/Blueprints/Characters/BP_Character_ADC.BP_Character_ADC_C" _returnvalue "AdjustIfPossibleButAlwaysSpawn" "OverrideRootScale" null null))
        (`PaperSpriteComponent.SetSprite` (`ENTCharacter.SpriteComponent` _returnvalue_4) "/Game/Sprites/Characters/RedADC_Sprite.RedADC_Sprite")
        (return _returnvalue_4))
      (:`1`
        (bind _returnvalue_5 (`|SpawnActorFromClass` "/Game/Blueprints/Characters/BP_Character_ADC.BP_Character_ADC_C" _returnvalue "AdjustIfPossibleButAlwaysSpawn" "OverrideRootScale" null null))
        (`PaperSpriteComponent.SetSprite` (`ENTCharacter.SpriteComponent` _returnvalue_5) "/Game/Sprites/Characters/PinkADC_Sprite.PinkADC_Sprite")
        (return _returnvalue_5))
      (:`2`
        (bind _returnvalue_6 (`|SpawnActorFromClass` "/Game/Blueprints/Characters/BP_Character_ADC.BP_Character_ADC_C" _returnvalue "AdjustIfPossibleButAlwaysSpawn" "OverrideRootScale" null null))
        (`PaperSpriteComponent.SetSprite` (`ENTCharacter.SpriteComponent` _returnvalue_6) "/Game/Sprites/Characters/BlueADC_Sprite.BlueADC_Sprite")
        (return _returnvalue_6))
      (:`3`
        (bind _returnvalue_7 (`|SpawnActorFromClass` "/Game/Blueprints/Characters/BP_Character_ADC.BP_Character_ADC_C" _returnvalue "AdjustIfPossibleButAlwaysSpawn" "OverrideRootScale" null null))
        (`PaperSpriteComponent.SetSprite` (`ENTCharacter.SpriteComponent` _returnvalue_7) "/Game/Sprites/Characters/GreenADC_Sprite.GreenADC_Sprite")
        (return _returnvalue_7))
      (:`4`
        (bind _returnvalue_8 (`|SpawnActorFromClass` "/Game/Blueprints/Characters/BP_Character_Assassin.BP_Character_Assassin_C" _returnvalue "AdjustIfPossibleButAlwaysSpawn" "OverrideRootScale" null null))
        (`PaperSpriteComponent.SetSprite` (`ENTCharacter.SpriteComponent` _returnvalue_8) "/Game/Sprites/Characters/RedAssassin_Sprite.RedAssassin_Sprite")
        (return _returnvalue_8))
      (:`5`
        (bind _returnvalue_9 (`|SpawnActorFromClass` "/Game/Blueprints/Characters/BP_Character_Assassin.BP_Character_Assassin_C" _returnvalue "AdjustIfPossibleButAlwaysSpawn" "OverrideRootScale" null null))
        (`PaperSpriteComponent.SetSprite` (`ENTCharacter.SpriteComponent` _returnvalue_9) "/Game/Sprites/Characters/PinkAssassin_Sprite.PinkAssassin_Sprite")
        (return _returnvalue_9))
      (:`6`
        (bind _returnvalue_10 (`|SpawnActorFromClass` "/Game/Blueprints/Characters/BP_Character_Assassin.BP_Character_Assassin_C" _returnvalue "AdjustIfPossibleButAlwaysSpawn" "OverrideRootScale" null null))
        (`PaperSpriteComponent.SetSprite` (`ENTCharacter.SpriteComponent` _returnvalue_10) "/Game/Sprites/Characters/BlueAssassin_Sprite.BlueAssassin_Sprite")
        (return _returnvalue_10))
      (:`7`
        (bind _returnvalue_11 (`|SpawnActorFromClass` "/Game/Blueprints/Characters/BP_Character_Assassin.BP_Character_Assassin_C" _returnvalue "AdjustIfPossibleButAlwaysSpawn" "OverrideRootScale" null null))
        (`PaperSpriteComponent.SetSprite` (`ENTCharacter.SpriteComponent` _returnvalue_11) "/Game/Sprites/Characters/GreenAssassin_Sprite.GreenAssassin_Sprite")
        (return _returnvalue_11))
      (:`8`
        (bind _returnvalue_12 (`|SpawnActorFromClass` "/Game/Blueprints/Characters/BP_Character_Bruiser.BP_Character_Bruiser_C" _returnvalue "AdjustIfPossibleButAlwaysSpawn" "OverrideRootScale" null null))
        (`PaperSpriteComponent.SetSprite` (`ENTCharacter.SpriteComponent` _returnvalue_12) "/Game/Sprites/Characters/RedBruiser_Sprite.RedBruiser_Sprite")
        (return _returnvalue_12))
      (:`9`
        (bind _returnvalue_13 (`|SpawnActorFromClass` "/Game/Blueprints/Characters/BP_Character_Bruiser.BP_Character_Bruiser_C" _returnvalue "AdjustIfPossibleButAlwaysSpawn" "OverrideRootScale" null null))
        (`PaperSpriteComponent.SetSprite` (`ENTCharacter.SpriteComponent` _returnvalue_13) "/Game/Sprites/Characters/PinkBruiser_Sprite.PinkBruiser_Sprite")
        (return _returnvalue_13))
      (:`10`
        (bind _returnvalue_14 (`|SpawnActorFromClass` "/Game/Blueprints/Characters/BP_Character_Bruiser.BP_Character_Bruiser_C" _returnvalue "AdjustIfPossibleButAlwaysSpawn" "OverrideRootScale" null null))
        (`PaperSpriteComponent.SetSprite` (`ENTCharacter.SpriteComponent` _returnvalue_14) "/Game/Sprites/Characters/BlueBruiser_Sprite.BlueBruiser_Sprite")
        (return _returnvalue_14))
      (:`11`
        (bind _returnvalue_15 (`|SpawnActorFromClass` "/Game/Blueprints/Characters/BP_Character_Bruiser.BP_Character_Bruiser_C" _returnvalue "AdjustIfPossibleButAlwaysSpawn" "OverrideRootScale" null null))
        (`PaperSpriteComponent.SetSprite` (`ENTCharacter.SpriteComponent` _returnvalue_15) "/Game/Sprites/Characters/GreenBruiser_Sprite.GreenBruiser_Sprite")
        (return _returnvalue_15))
      (:`12`
        (bind _returnvalue_16 (`|SpawnActorFromClass` "/Game/Blueprints/Characters/BP_Character_Tank.BP_Character_Tank_C" _returnvalue "AdjustIfPossibleButAlwaysSpawn" "OverrideRootScale" null null))
        (`PaperSpriteComponent.SetSprite` (`ENTCharacter.SpriteComponent` _returnvalue_16) "/Game/Sprites/Characters/RedTank_Sprite.RedTank_Sprite")
        (return _returnvalue_16))
      (:`13`
        (bind _returnvalue_17 (`|SpawnActorFromClass` "/Game/Blueprints/Characters/BP_Character_Bruiser.BP_Character_Bruiser_C" _returnvalue "AdjustIfPossibleButAlwaysSpawn" "OverrideRootScale" null null))
        (`PaperSpriteComponent.SetSprite` (`ENTCharacter.SpriteComponent` _returnvalue_17) "/Game/Sprites/Characters/PinkTank_Sprite.PinkTank_Sprite")
        (return _returnvalue_17))
      (:`14`
        (bind _returnvalue_18 (`|SpawnActorFromClass` "/Game/Blueprints/Characters/BP_Character_Bruiser.BP_Character_Bruiser_C" _returnvalue "AdjustIfPossibleButAlwaysSpawn" "OverrideRootScale" null null))
        (`PaperSpriteComponent.SetSprite` (`ENTCharacter.SpriteComponent` _returnvalue_18) "/Game/Sprites/Characters/BlueTank_Sprite.BlueTank_Sprite")
        (return _returnvalue_18))
      (:`15`
        (bind _returnvalue_19 (`|SpawnActorFromClass` "/Game/Blueprints/Characters/BP_Character_Bruiser.BP_Character_Bruiser_C" _returnvalue "AdjustIfPossibleButAlwaysSpawn" "OverrideRootScale" null null))
        (`PaperSpriteComponent.SetSprite` (`ENTCharacter.SpriteComponent` _returnvalue_19) "/Game/Sprites/Characters/GreenTank_Sprite.GreenTank_Sprite")
        (return _returnvalue_19)))))

(fn `UserConstructionScript`)